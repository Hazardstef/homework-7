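; BP_Materials is an actor Blueprint that changes the material of its Cube when another actor begins overlapping it.
; The overlap event calls the parent, then sets TutorialMaterial on the cube's first slot, with no filter on the other actor and no revert.
; BeginPlay checks that Cube is valid but acts on neither result, Tick is disabled, and the construction script only calls its parent.
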(event `self.ReceiveBeginPlay`
  (`parent.ReceiveBeginPlay`)
  (`/Engine/EditorBlueprintResources/StandardMacros.IsValid` (`self.Cube`)))

(event `self.ReceiveActorBeginOverlap`
  (params (OtherActor :type "Actor Object Reference"))
  (`parent.ReceiveActorBeginOverlap` OtherActor)
  (`PrimitiveComponent.SetMaterial` (`self.Cube`) 0 "/Engine/Tutorial/SubEditors/TutorialAssets/TutorialMaterial.TutorialMaterial"))

(fn `UserConstructionScript`
  (`parent.UserConstructionScript`))