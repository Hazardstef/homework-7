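; BP_Sphere is an actor that moves at a set speed and bounces off whatever blocks it.
; Each tick it makes a swept world-offset move along Direction, scaled by Speed and frame time.
; On a blocking hit it reflects Direction about the surface normal, zeroes Z to keep travel horizontal, and prints a debug string.
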(event `self.ReceiveTick`
  (params (DeltaSeconds :type "Float (single-precision)"))
  (bind _sweephitresult (`self.K2_AddActorWorldOffset` (* DeltaSeconds (* (`self.speed`) (`self.direction`))) true))
  (bind (_bblockinghit _binitialoverlap _time _distance _location _impactpoint _normal) (`GameplayStatics.BreakHitResult` _sweephitresult))
  (if _bblockinghit
    (bind (_returnvalue_x _returnvalue_y) (`KismetMathLibrary.BreakVector` (`KismetMathLibrary.GetReflectionVector` (`self.direction`) _normal)))
    (set `self.direction` (`KismetMathLibrary.MakeVector` _returnvalue_x _returnvalue_y))
    (`KismetSystemLibrary.PrintString` "Hello")))

(fn `UserConstructionScript`)