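; BP_Scale is an actor that shrinks by five percent each time another actor begins overlapping it.
; The overlap event multiplies the current actor scale, so the reduction compounds with no lower limit or filter on the other actor, and prints a debug message.
; BeginPlay only runs an unused validity check on Cube, and Tick is disabled.
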(event `self.ReceiveBeginPlay`
  (`parent.ReceiveBeginPlay`)
  (`/Engine/EditorBlueprintResources/StandardMacros.IsValid` (`self.Cube`)))

(event `self.ReceiveActorBeginOverlap`
  (params (OtherActor :type "Actor Object Reference"))
  (`parent.ReceiveActorBeginOverlap` OtherActor)
  (bind _output_get (set `self.size` (`self.GetActorScale3D`)))
  (bind _output_get_2 (set `self.size` (* _output_get (0.95 0.95 0.95))))
  (`self.SetActorScale3D` _output_get_2)
  (`KismetSystemLibrary.PrintString` "size -5%"))

(fn `UserConstructionScript`
  (`parent.UserConstructionScript`))